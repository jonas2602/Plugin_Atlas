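; AtlasGM_BP is an Atlas system Blueprint that currently acts as a scratchpad for transform math, with no gameplay logic.
; On BeginPlay it prints the result of MakeRelativeTransform on two hard-coded transforms, expressing one in the space of the other.
; Unconnected nodes try related operations on similar sample values: transforming and inverse-transforming locations and directions, inverting a transform, and rotator math.
; The construction script is empty.
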(event EventBeginPlay
  (Development|PrintString (Utilities|String|ToString(Transform) (Math|Transform|MakeRelativeTransform (Math|Transform|MakeTransform "1.000000,2.000000,0.000000" "0.000000,-90.000000,0.000000" "0.750000,0.750000,0.750000") (Math|Transform|MakeTransform "4.000000,3.000000,0.000000" "0.000000,45.000000,0.000000" "0.500000,0.500000,0.500000")))))

(fn ConstructionScript)