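; Atlas_3D_BP is the 3D view of the Atlas storage, showing each storage entry as a spawned figure actor.
; On BeginPlay it binds to the storage's add and remove events and creates figures for existing entries.
; Each figure attaches under EntryRoot, connects to its entry, receives player input and is mapped by entry for removal.
; Figure transform-change events update relative location and rotation while keeping scale.
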(event Custom|RemoveEntry
  (params (StorageEntry :type Atlas%20Storage%20Entry%20Object%20Reference))
  (Actor|DestroyActor (.Value (Utilities|Map|Find (Variables|Default|GetStorageEntryMap) StorageEntry)))
  (Utilities|Map|Remove (Variables|Default|GetStorageEntryMap) StorageEntry))

(event Custom|AddEntry
  (params (StorageEntry :type Atlas%20Storage%20Entry%20Object%20Reference))
  (bind _returnvalue (Game|SpawnActorfromClass (Variables|/Script/AtlasSystem.AtlasStorageEntry|GetEntryFigureClass StorageEntry) (Math|Transform|MakeTransform "0, 0, 0" "0, 0, 0" "5.000000,5.000000,5.000000") "Undefined" 0 0))
  (Transformation|AttachComponentToComponent _returnvalue (Variables|Default|GetEntryRoot) "None" "SnapToTarget" "SnapToTarget" "KeepWorld" true)
  (bind _asatlas_figure_bp (Utilities|Casting|CastToAtlasFigure_BP _returnvalue))
  (EventDispatchers|BindEventtoOnDesiredTransformChanged _asatlas_figure_bp (EventDispatchers|CreateEvent :!event Custom|OnStorageTransformChanged))
  (Default|ConnectStorageEntry _asatlas_figure_bp StorageEntry)
  (Input|EnableInput _asatlas_figure_bp (Game|GetPlayerController 0))
  (Utilities|Map|Add (Variables|Default|GetStorageEntryMap) StorageEntry _asatlas_figure_bp))

(event Custom|OnStorageTransformChanged
  (params (Figure :type Atlas%20Entry%20Figure%20Object%20Reference) (Transform :type Transform%20%28by%20ref%29))
  (Transformation|SetActorRelativeTransform Figure (Math|Transform|MakeTransform (.location Transform) (.rotation Transform) (Class|Actor|GetActorRelativeScale3D Figure)) false true))

(event EventBeginPlay
  (bind _returnvalue (Class|AtlasBlueprintLibrary|GetAtlasStorage))
  (EventDispatchers|BindEventtoOnStorageEntryAdded _returnvalue (EventDispatchers|CreateEvent :!event Custom|AddEntry))
  (EventDispatchers|BindEventtoOnStorageEntryRemoved _returnvalue (EventDispatchers|CreateEvent :!event Custom|RemoveEntry))
  (for _array_element (Class|AtlasStorage|GetStorageEntries _returnvalue)
    (CallFunction|AddEntry _array_element)))

(fn ConstructionScript)