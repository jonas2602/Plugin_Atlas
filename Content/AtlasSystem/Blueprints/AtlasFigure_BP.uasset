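; Atlas figure actor that displays a mesh from its storage entry and responds to the cursor.
; On storage state change, it casts the entry to ImageStorageEntry and applies its mesh and relative scale.
; Hovering toggles custom depth rendering on the mesh, while clicking only prints a test message.
; It supplies a TooltipContent_WB widget with placeholder text; bounds debug drawing and a Landscape cast are left unconnected.
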(event MouseInput|EventActorBeginCursorOver
  (Rendering|SetRenderCustomDepth (Variables|Default|GetStaticMesh) true))

(event MouseInput|EventActorEndCursorOver
  (Rendering|SetRenderCustomDepth (Variables|Default|GetStaticMesh) false))

(event EventOnStorageStateChanged
  (bind _asimage_storage_entry (Utilities|Casting|CastToImageStorageEntry (Variables|Default|GetStorageEntry)))
  (Components|StaticMesh|SetStaticMesh (Variables|Default|GetStaticMesh) (Variables|/Game/AtlasSystem/Blueprints/ImageStorageEntry.ImageStorageEntry_C|GetMesh _asimage_storage_entry))
  (Transformation|SetActorRelativeScale3D (Variables|/Game/AtlasSystem/Blueprints/ImageStorageEntry.ImageStorageEntry_C|GetMeshSize _asimage_storage_entry)))

(event MouseInput|EventActorOnClicked
  (params (ButtonPressed :type Key%20Structure))
  (Development|PrintString "Hello"))

(fn ConstructionScript)

(fn CreateTooltipContent
  (bind _returnvalue (UserInterface|CreateWidget "/Game/AtlasSystem/Widgets/TooltipContent_WB.TooltipContent_WB_C" (Game|GetPlayerController 0) "test 23"))
  (return _returnvalue))