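; Debug test actor in the Atlas System that compares ways of projecting its own world location to screen space.
; Each Tick it logs, without printing on screen, its widget-space position, its player-viewport-relative screen position for player 0, and the viewport size.
; An unconnected Append retains a wider comparison that adds non-relative and PlayerController projection variants.
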(event EventBeginPlay)

(event Collision|EventActorBeginOverlap
  (params (OtherActor :type Actor%20Object%20Reference)))

(event EventTick
  (params (DeltaSeconds :type Float%20%28single-precision%29))
  (bind _returnvalue (Game|GetPlayerController 0))
  (bind _returnvalue_2 (Transformation|GetActorLocation))
  (Development|PrintString (Utilities|String|Append "WorldToWidget: " (Utilities|String|ToString(Vector2d) (.ScreenPosition (Class|WidgetLayoutLibrary|ProjectWorldLocationtoWidgetPosition _returnvalue _returnvalue_2))) ",       WorldToScreen(true): " (Utilities|String|ToString(Vector2d) (.ScreenPosition (Class|GameplayStatics|ProjectWorldtoScreen _returnvalue _returnvalue_2 true)))) false)
  (Development|PrintString (Utilities|String|Append "Viewport: " (Utilities|String|ToString(Vector2d) (Viewport|GetViewportSize))) false))

(fn ConstructionScript)