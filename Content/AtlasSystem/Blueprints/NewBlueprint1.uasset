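; NewBlueprint1 is an actor with a capsule that appears to be a scratch test for movement and location reporting.
; On BeginPlay it sets the capsule radius, and only the instance named NewBlueprint2 then waits, offsets itself without sweep and prints its location before and after, plus the hit actor.
; That instance's Tick caches its location and prints it whenever it changes.
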(event EventBeginPlay
  (Components|Capsule|SetCapsuleRadius (Variables|Default|GetCapsule) 5e+01 true)
  (if (Utilities|Enum|Equal(Enum) (Utilities|GetDisplayName self) "NewBlueprint2")
    (Utilities|FlowControl|Delay 2.0)
    (Development|PrintString (Utilities|String|ToString(Vector) (Transformation|GetActorLocation)))
    (bind _sweephitresult (Transformation|AddActorWorldOffset "-260.000000, 0,1.000000"))
    (Development|PrintString (Utilities|GetDisplayName (.HitActor (Collision|BreakHitResult _sweephitresult))))
    (Development|PrintString (Utilities|String|ToString(Vector) (Transformation|GetActorLocation)))
    (Utilities|FlowControl|Delay 0.016)
    (Development|PrintString (Utilities|String|ToString(Vector) (Transformation|GetActorLocation)))))

(event Collision|EventActorBeginOverlap
  (params (OtherActor :type Actor%20Object%20Reference)))

(event EventTick
  (params (DeltaSeconds :type Float%20%28single-precision%29))
  (bind _returnvalue (Transformation|GetActorLocation))
  (if (and (Utilities|Enum|Equal(Enum) (Utilities|GetDisplayName self) "NewBlueprint2") (Math|Vector|NotEqual(Vector) _returnvalue (Variables|Default|GetNewVar_0) 0.0001))
    (Development|PrintString (Utilities|String|ToString(Vector) _returnvalue))
    (Variables|Default|SetNewVar_0 _returnvalue)))

(fn ConstructionScript)